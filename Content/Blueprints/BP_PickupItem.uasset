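; World pickup for a weapon, offered to any SCharacter that overlaps it.
; On BeginPlay it spawns an instance of WeaponClass at its own location, hides it in game and stores it in WeaponItem.
; It copies that weapon's skeletal mesh onto InnerMesh for display.
; On overlap it passes itself to the character's Pickup function, which handles the rest.
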(event EventBeginPlay
  (if (Utilities|IsValidClass (Variables|Default|GetWeaponClass))
    (bind _weaponitem (CallFunction|CreateItem))
    (CallFunction|SetWeaponSkeletalMesh _weaponitem)))

(event Collision|EventActorBeginOverlap
  (params (OtherActor :type Actor%20Object%20Reference))
  (bind _asscharacter (Utilities|Casting|CastToSCharacter OtherActor))
  (Class|SCharacter|Pickup _asscharacter self))

(fn ConstructionScript)

(fn CreateItem
  (bind _returnvalue (Game|SpawnActorfromClass (Variables|Default|GetWeaponClass) (Math|Transform|MakeTransform (Transformation|GetActorLocation)) "AlwaysSpawn" 0 0))
  (Utilities|IsValid _returnvalue
    (:Is%20Valid
      (Rendering|SetActorHiddenInGame _returnvalue true)
      (bind _output_get (Variables|Default|SetWeaponItem _returnvalue))
      (return _output_get))))

(fn SetWeaponSkeletalMesh
  (params (WeaponItem :type S%20Weapon%20Object%20Reference))
  (bind _meshcomponent (Variables|/Script/CoopGame.SWeapon|GetMeshComponent WeaponItem))
  (bind _skeletalmesh (Variables|/Script/Engine.SkinnedMeshComponent|GetSkeletalMesh _meshcomponent))
  (Utilities|IsValid WeaponItem
    (:Is%20Valid
      (Utilities|IsValid _skeletalmesh
        (:Is%20Valid
          (Class|SkinnedMeshComponent|SetSkeletalMesh (Variables|Default|GetInnerMesh) _skeletalmesh false))))))