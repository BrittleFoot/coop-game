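; Player character Blueprint that sets up the basic HUD and reacts physically to radial damage.
; On BeginPlay, only the locally controlled instance creates the crosshair and health indicator widgets and adds them to the viewport.
; Radial damage applies a velocity-change impulse to CharacterMovement along the negated hit impact normal, scaled by damage received, producing knockback.
; The Blueprint does no health bookkeeping, and its construction script is empty.
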(event EventBeginPlay
  ;[1 1 1] Create Default UI
  (if (Pawn|IsLocallyControlled)
    (Utilities|FlowControl|Sequence
      (:then_0
        (bind _returnvalue (UserInterface|CreateWidget "/Game/UI/WBP_Crosshair.WBP_Crosshair_C"))
        (UserInterface|Viewport|AddtoViewport _returnvalue 0))
      (:then_1
        (bind _returnvalue_2 (UserInterface|CreateWidget "/Game/UI/WBP_HealthIndicator.WBP_HealthIndicator_C"))
        (UserInterface|Viewport|AddtoViewport _returnvalue_2 0)))))

(event Game|Damage|EventRadialDamage
  (params (DamageReceived :type Float%20%28single-precision%29) (DamageType :type Damage%20Type%20Object%20Reference) (Origin :type Vector :default "0, 0, 0") (HitInfo :type Hit%20Result%20Structure%20%28by%20ref%29) (InstigatedBy :type Controller%20Object%20Reference) (DamageCauser :type Actor%20Object%20Reference))
  ;[1 1 1] Radial Damage Impact
  (Physics|AddImpulse (Variables|Character|GetCharacterMovement) (* (.ImpactNormal (Collision|BreakHitResult HitInfo)) (* DamageReceived -1e+01)) true))

(fn ConstructionScript)